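; BP_Stamat is an AI-controlled actor named Stamat that can be toggled to follow another actor.
; On BeginPlay it caches its AI_Stamat controller.
; The Follow event flips IsFollowing and switches the controller's Stamat state, passing the actor to follow when following starts.
; The Target event takes a location but is empty, as is the construction script.
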(event `self.ReceiveBeginPlay`
  ;[1 1 1] Enable controls
  (bind _asai_stamat (cast `/Game/Stamat/AI_Stamat` (`AIBlueprintHelperLibrary.GetAIController` self)))
  (set `self.StamatController` _asai_stamat))

(event `Follow`
  (params (FollowActor :type "Actor Object Reference"))
  ;[1 1 1] Follow
  (if (`self.IsFollowing`)
    (`/Game/Stamat/AI_Stamat.SetStamatState` (`self.StamatController`) "NewEnumerator0")
    (set `self.IsFollowing` false)
    (else
      (`/Game/Stamat/AI_Stamat.FollowActor` (`self.StamatController`) FollowActor)
      (`/Game/Stamat/AI_Stamat.SetStamatState` (`self.StamatController`) "NewEnumerator1")
      (set `self.IsFollowing` true))))

(event `Target`
  (params (Location :type "Vector Structure")))

(fn `UserConstructionScript`)